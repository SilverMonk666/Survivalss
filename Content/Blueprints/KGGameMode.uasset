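; Game mode that runs wave-based enemy spawning and ends the game after the last wave.
; A looping timer spawns enemies from the current wave's shuffled class queue at random PlayerStart positions.
; Enemy destruction starts the next wave once the queue is empty and no KGAIControllerBase actors remain.
; New-wave and endgame dispatchers fire on transitions, and endgame blends to a random CameraActor before restarting the level.
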(event `self.ReceiveBeginPlay`
  (`KismetSystemLibrary.K2_SetTimerDelegate` (delegate `SpawnEnemy`) 1.0 true)
  (`self.ResetGame`))

(event `SpawnEnemy`
  (if (> (`KismetArrayLibrary.Array_Length` (`self.CurrentCue`)) 0)
    (bind _outactors (`GameplayStatics.GetAllActorsOfClass` "/Script/Engine.PlayerStart"))
    (bind _output (`|GetArrayItem` _outactors (`KismetMathLibrary.RandomInteger` (`KismetArrayLibrary.Array_Length` _outactors))))
    (bind _returnvalue (`AIBlueprintHelperLibrary.SpawnAIFromClass` (`|GetArrayItem` (`self.CurrentCue`)) null (`self.K2_GetActorLocation` _output) (`self.K2_GetActorRotation` _output)))
    (`KismetArrayLibrary.Array_Remove` (`self.CurrentCue`))
    (add `self.OnDestroyed` _returnvalue (delegate `CheckWaveComplete`))))

(event `CheckWaveComplete` :!signature `self.OnDestroyed`
  (params (DestroyedActor :type "Actor Object Reference"))
  (if (== (`KismetArrayLibrary.Array_Length` (`self.CurrentCue`)) 0)
    (bind _outactors (`GameplayStatics.GetAllActorsOfClass` "/Game/Blueprints/KGAIControllerBase.KGAIControllerBase_C"))
    (if (== (`KismetArrayLibrary.Array_Length` _outactors) 0)
      (`self.StartNewWave`))))

(event `ResetGame`
  (bind _output_classtospawn (break `/Game/Blueprints/WaveStruct` (`|GetArrayItem` (`self.Waves`) (`self.WaveIndex`))))
  (set `self.WaveIndex` 0)
  (bind _output_get (set `self.CurrentCue` _output_classtospawn :!label _label))
  (`KismetArrayLibrary.Array_Shuffle` _output_get))

(event `StartNewWave`
  (`/Engine/EditorBlueprintResources/StandardMacros.IncrementInt` (`self.WaveIndex`)
    (:`  `
      (`self.NewWave`)
      (if (< (`KismetArrayLibrary.Array_LastIndex` (`self.Waves`)) (`self.WaveIndex`))
        (`self.Endgame`)
        (else
          (goto _label))))))

(event `Endgame`
  (`self.EndgameDispatcher`)
  (bind _outactors (`GameplayStatics.GetAllActorsOfClass` "/Script/Engine.CameraActor"))
  (`KismetSystemLibrary.PrintString` "JustAbout")
  (`PlayerController.SetViewTargetWithBlend` (`GameplayStatics.GetPlayerController` 0) (`|GetArrayItem` _outactors (`KismetMathLibrary.RandomInteger` (`KismetArrayLibrary.Array_Length` _outactors))) 4.0 "VTBlend_Linear" 0.0 true)
  (`KismetSystemLibrary.PrintString` "Happened")
  (`KismetSystemLibrary.Delay` 6.0)
  (`KismetSystemLibrary.ExecuteConsoleCommand` "restartlevel"))

(fn `UserConstructionScript`)